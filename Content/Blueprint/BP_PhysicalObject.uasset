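; BP_PhysicalObject is a data-driven sprite object whose appearance and Tag come from the DT_PhysicalObject data table.
; The construction script looks up the row named by ObjectGame, then sets the render component's sprite and stores the row's Tag.
; An Update event repeats the same lookup for a passed-in ObjectName, allowing the object's sprite and Tag to be swapped after construction.
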(event `Update`
  (params (ObjectName :type String))
  (bind _returnvalue (`|GetDataTableRow` "/Game/DataTables/PhysicalObject/DT_PhysicalObject.DT_PhysicalObject" (`KismetStringLibrary.Conv_StringToName` ObjectName))
    (:`then`
      (bind (_tag _sprite) (break `/Game/DataTables/PhysicalObject/STR_PhysicalObject` _returnvalue))
      (`PaperSpriteComponent.SetSprite` (`self.RenderComponent1`) _sprite)
      (set `self.Tag` _tag))))

(fn `UserConstructionScript`
  (bind _returnvalue (`|GetDataTableRow` "/Game/DataTables/PhysicalObject/DT_PhysicalObject.DT_PhysicalObject" (`self.ObjectGame`))
    (:`then`
      (bind (_tag _sprite) (break `/Game/DataTables/PhysicalObject/STR_PhysicalObject` _returnvalue))
      (`PaperSpriteComponent.SetSprite` (`self.RenderComponent1`) _sprite)
      (set `self.Tag` _tag))))